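; Lighting_control is a Blueprint that runs the lighting transition from menu to show when ShowTime is called, using tagged spotlights.
; On BeginPlay it stores a reference to the top-level UI widget.
; ShowTime runs delayed timelines that drive the intensity of menu lights, then front and back lights.
; After a longer delay it unhides either the one-player or the default spotlights, based on the UI's SinglePlayer flag.
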(event `self.ReceiveBeginPlay`
  (bind _foundwidgets (`WidgetBlueprintLibrary.GetAllWidgetsOfClass` "/Game/Blueprints/UI.UI_C"))
  (for _array_element _foundwidgets
    (set `self.Ui` _array_element)))

(event `ShowTime`
  (`|ExecutionSequence`
    (:`then_0`
      (`KismetSystemLibrary.Delay` 1.0)
      (bind _outactors (`GameplayStatics.GetAllActorsOfClassWithTag` "/Script/Engine.SpotLight" "Menu_Lights"))
      (bind (_direction _intensity) (`Timeline|ReduceInsintiy` :!via `PlayFromStart`)
        (:`Update`
          (for _array_element _outactors
            (`LightComponent.SetIntensity` (`Light.LightComponent` _array_element) _intensity)))))
    (:`then_1`
      (`KismetSystemLibrary.Delay` 2.0)
      (`|ExecutionSequence`
        (:`then_0`
          (bind _outactors_2 (`GameplayStatics.GetAllActorsOfClassWithTag` "/Script/Engine.SpotLight" "Front Lights"))
          (bind (_direction_2 _intensity_2) (`Timeline|Increase intesity`)
            (:`Update`
              (for _array_element_2 _outactors_2
                (`LightComponent.SetIntensity` (`Light.LightComponent` _array_element_2) _intensity_2)))))
        (:`then_1`
          (bind _outactors_3 (`GameplayStatics.GetAllActorsOfClassWithTag` "/Script/Engine.SpotLight" "Back_light"))
          (bind (_direction_3 _intensity_3) (`Timeline|Timeline`)
            (:`Update`
              (for _array_element_3 _outactors_3
                (`LightComponent.SetIntensity` (`Light.LightComponent` _array_element_3) _intensity_3)))))))
    (:`then_2`
      (if (`/Game/Blueprints/UI.SinglePlayer` (`self.Ui`))
        (`KismetSystemLibrary.Delay` 7.0)
        (bind _outactors_4 (`GameplayStatics.GetAllActorsOfClassWithTag` "/Script/Engine.SpotLight" "Spot_Light_1p"))
        (for _array_element_4 _outactors_4
          (`self.SetActorHiddenInGame` _array_element_4 false))
        (else
          (`KismetSystemLibrary.Delay` 7.0)
          (bind _outactors_5 (`GameplayStatics.GetAllActorsOfClassWithTag` "/Script/Engine.SpotLight" "Spot_Light"))
          (for _array_element_5 _outactors_5
            (`self.SetActorHiddenInGame` _array_element_5 false)))))))

(fn `UserConstructionScript`)