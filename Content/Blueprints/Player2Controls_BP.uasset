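; Player 2 controls Blueprint that receives the four directional inputs (up, down, left, right) for a two-player game mode.
; On BeginPlay it adds the controls mapping context to its player controller's Enhanced Input subsystem.
; Each input checks the UI widget's game-started and two-player flags, then casts the parent actor to Player2Arrow_BP.
; The branches after those casts are empty, as are the IncreaseScore and ResetCombo events.
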(event `self.ReceiveBeginPlay`
  ;[1 1 1] Set Inputs
  (bind _asplayer_controller (cast `PlayerController` (`self.GetController`)))
  (bind _returnvalue (pcsubsystem `EnhancedInputLocalPlayerSubsystem` _asplayer_controller))
  (`/Engine/EditorBlueprintResources/StandardMacros.IsValid` _returnvalue
    (:`Is Valid`
      (`EnhancedInputSubsystemInterface.AddMappingContext` _returnvalue "/Game/Inputs/ControlsInputMapping.ControlsInputMapping" 0 (struct)))))

(event `EnhancedInput|/Game/Inputs/IA_Player2Down`
  (params (ActionValue :type Boolean) (ElapsedSeconds :type "Float (double-precision)") (TriggeredSeconds :type "Float (double-precision)") (InputAction :type "InputAction Object Reference" :default "/Game/Inputs/IA_Player2Down.IA_Player2Down"))
  (:`Started`
    (bind _foundwidgets (`WidgetBlueprintLibrary.GetAllWidgetsOfClass` "/Game/Blueprints/UI.UI_C"))
    (bind _output (`|GetArrayItem` _foundwidgets))
    (if (and (`/Game/Blueprints/UI.GameStarted` _output) (`/Game/Blueprints/UI.2PlayerGame` _output))
      (cast `/Game/Blueprints/Player2Arrow_BP` (`self.GetParentActor`))
      (if true
        _))))

(event `EnhancedInput|/Game/Inputs/IA_Player2Left`
  (params (ActionValue :type Boolean) (ElapsedSeconds :type "Float (double-precision)") (TriggeredSeconds :type "Float (double-precision)") (InputAction :type "InputAction Object Reference" :default "/Game/Inputs/IA_Player2Left.IA_Player2Left"))
  (:`Started`
    (bind _foundwidgets (`WidgetBlueprintLibrary.GetAllWidgetsOfClass` "/Game/Blueprints/UI.UI_C"))
    (bind _output (`|GetArrayItem` _foundwidgets))
    (if (and (`/Game/Blueprints/UI.GameStarted` _output) (`/Game/Blueprints/UI.2PlayerGame` _output))
      (cast `/Game/Blueprints/Player2Arrow_BP` (`self.GetParentActor`))
      (if true
        _))))

(event `EnhancedInput|/Game/Inputs/IA_Player2Right`
  (params (ActionValue :type Boolean) (ElapsedSeconds :type "Float (double-precision)") (TriggeredSeconds :type "Float (double-precision)") (InputAction :type "InputAction Object Reference" :default "/Game/Inputs/IA_Player2Right.IA_Player2Right"))
  (:`Started`
    (bind _foundwidgets (`WidgetBlueprintLibrary.GetAllWidgetsOfClass` "/Game/Blueprints/UI.UI_C"))
    (bind _output (`|GetArrayItem` _foundwidgets))
    (if (and (`/Game/Blueprints/UI.GameStarted` _output) (`/Game/Blueprints/UI.2PlayerGame` _output))
      (cast `/Game/Blueprints/Player2Arrow_BP` (`self.GetParentActor`))
      (if true
        _))))

(event `EnhancedInput|/Game/Inputs/IA_Player2Up`
  (params (ActionValue :type Boolean) (ElapsedSeconds :type "Float (double-precision)") (TriggeredSeconds :type "Float (double-precision)") (InputAction :type "InputAction Object Reference" :default "/Game/Inputs/IA_Player2Up.IA_Player2Up"))
  (:`Started`
    (bind _foundwidgets (`WidgetBlueprintLibrary.GetAllWidgetsOfClass` "/Game/Blueprints/UI.UI_C"))
    (bind _output (`|GetArrayItem` _foundwidgets))
    (if (and (`/Game/Blueprints/UI.GameStarted` _output) (`/Game/Blueprints/UI.2PlayerGame` _output))
      (cast `/Game/Blueprints/Player2Arrow_BP` (`self.GetParentActor`))
      (if true
        _))))

(event `IncreaseScore`)

(event `ResetCombo`)

(fn `UserConstructionScript`)