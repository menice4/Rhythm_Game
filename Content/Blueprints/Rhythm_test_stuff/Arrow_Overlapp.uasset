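; Rhythm-game test actor whose box detects overlapping arrows tagged with its Direction and times them with a decaying score.
; A matching overlap stores the arrow and opens a gated delay loop that counts Score down from its starting value.
; Any end overlap records a zero NewScore, resets Score, then destroys the stored arrow and closes the gate.
; An unconnected branch would record the current Score while overlapping.
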(event `self.ReceiveBeginPlay`
  (set `self.Score` 100.0))

(event `self.Box.OnComponentBeginOverlap`
  (params (OverlappedComponent :type "PrimitiveComponent Object Reference") (OtherActor :type "Actor Object Reference") (OtherComp :type "PrimitiveComponent Object Reference") (OtherBodyIndex :type Integer) (bFromSweep :type Boolean) (SweepResult :type "HitResult Structure (by ref)"))
  (if (`self.ActorHasTag` OtherActor (`self.Direction`))
    (set `self.Collide` OtherActor)
    (set `self.Is Overlapping` true)
    (`|ExecutionSequence`
      (:`then_0`
        (goto _label :!via `Open`))
      (:`then_1`
        (`/Engine/EditorBlueprintResources/StandardMacros.Gate` true :!label _label
          (:`Exit`
            (set `self.Score` (- (`self.Score`) 1.0))
            (`KismetSystemLibrary.Delay` 0.1)
            (goto _label)))))))

(event `self.Box.OnComponentEndOverlap`
  (params (OverlappedComponent :type "PrimitiveComponent Object Reference") (OtherActor :type "Actor Object Reference") (OtherComp :type "PrimitiveComponent Object Reference") (OtherBodyIndex :type Integer))
  (bind _collide (`self.Collide`))
  (set `self.Score` 0.0)
  (set `self.New_score` (`self.Score`))
  (set `self.Score` 100.0)
  (set `self.Is Overlapping` false)
  (`/Engine/EditorBlueprintResources/StandardMacros.IsValid` _collide
    (:`Is Valid`
      (`self.K2_DestroyActor` _collide)
      (`KismetSystemLibrary.PrintString` "Hello")
      (goto _label :!via `Close`))))

(fn `UserConstructionScript`)