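; Player 1 arrow hit zone for a rhythm minigame, scoring key presses while an arrow overlaps its Box.
; A Gate and Delay loop counts the score down from ten during overlap; the matching key submits it, while a wrong key or end of overlap scores zero.
; Each result goes to Rythum_Master_BP, then the arrow is destroyed.
; A Back_up volume destroys anything entering it, and SetRotation offsets the plane's yaw at BeginPlay.
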(event `self.ReceiveBeginPlay`
  (bind _plane (`self.Plane`))
  (bind (_returnvalue_roll _returnvalue_pitch _returnvalue_yaw) (`KismetMathLibrary.BreakRotator` (`SceneComponent.K2_GetComponentRotation` _plane)))
  (set `self.Score_P1` 10.0)
  (bind _returnvalue (`GameplayStatics.GetActorOfClass` "/Game/Blueprints/Rhythm_test_stuff/Rythum_Master_BP.Rythum_Master_BP_C"))
  (set `self.RythumMaster` _returnvalue)
  (`SceneComponent.K2_SetRelativeRotation` _plane (`KismetMathLibrary.MakeRotator` _returnvalue_roll _returnvalue_pitch (+ _returnvalue_yaw (`self.Set rotation`))) false false))

(event `self.Box.OnComponentBeginOverlap`
  (params (OverlappedComponent :type "PrimitiveComponent Object Reference") (OtherActor :type "Actor Object Reference") (OtherComp :type "PrimitiveComponent Object Reference") (OtherBodyIndex :type Integer) (bFromSweep :type Boolean) (SweepResult :type "HitResult Structure (by ref)"))
  (set `self.Collide` OtherActor)
  (set `self.Is Overlapping` true)
  (`|ExecutionSequence`
    (:`then_0`
      (goto _label :!via `Open`))
    (:`then_1`
      (`/Engine/EditorBlueprintResources/StandardMacros.Gate` true :!label _label
        (:`Exit`
          (set `self.Score_P1` (- (`self.Score_P1`) 1.0))
          (`KismetSystemLibrary.Delay` 0.1)
          (goto _label))))))

(event `self.Back_up.OnComponentBeginOverlap`
  (params (OverlappedComponent :type "PrimitiveComponent Object Reference") (OtherActor :type "Actor Object Reference") (OtherComp :type "PrimitiveComponent Object Reference") (OtherBodyIndex :type Integer) (bFromSweep :type Boolean) (SweepResult :type "HitResult Structure (by ref)"))
  (`self.K2_DestroyActor` OtherActor))

(event `self.Box.OnComponentEndOverlap`
  (params (OverlappedComponent :type "PrimitiveComponent Object Reference") (OtherActor :type "Actor Object Reference") (OtherComp :type "PrimitiveComponent Object Reference") (OtherBodyIndex :type Integer))
  (bind _collide (`self.Collide`))
  (bind _rythummaster (`self.RythumMaster`))
  (set `self.Score_P1` 0.0 :!label _label_2)
  (bind _output_get (set `self.Finale_score_P1` (`self.Score_P1`) :!label _label_3))
  (set `/Game/Blueprints/Rhythm_test_stuff/Rythum_Master_BP.P1_Score` (`KismetMathLibrary.FTrunc` _output_get) _rythummaster)
  (`/Game/Blueprints/Rhythm_test_stuff/Rythum_Master_BP.Score` _rythummaster)
  (set `self.Score_P1` 10.0)
  (set `self.Is Overlapping` false)
  (`/Engine/EditorBlueprintResources/StandardMacros.IsValid` _collide
    (:`Is Valid`
      (`self.K2_DestroyActor` _collide)
      (goto _label :!via `Close`))
    (:`Is Not Valid`
      (goto _label :!via `Close`))))

(event `Button pressed P1`
  (params (Key :type "Key Structure" :default "None"))
  (if (`self.Is Overlapping`)
    (if (== Key (`self.Key_required`))
      (`KismetSystemLibrary.PrintString` "working")
      (goto _label_3)
      (else
        (goto _label_2)))))

(event `/Game/Blueprints/Rhythm_test_stuff/Triggers.Button Press`
  (params (key :type "Key Structure")))

(fn `UserConstructionScript`)