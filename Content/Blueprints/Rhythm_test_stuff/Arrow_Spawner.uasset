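; Arrow spawner for a rhythm test that creates moving arrows in one of four direction lanes.
; Each Spawn_arrow call picks a random index and spawns an Arrow_moveing at half scale at the matching Up, Right, Left or Down component location.
; A step that sets a direction tag from the same index is disconnected and never runs.
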(event `Spawn_arrow`
  (set `self.RandomNum` (`KismetMathLibrary.RandomIntegerInRange` 0 3))
  (`|SpawnActorFromClass` "/Game/Blueprints/Rhythm_test_stuff/Arrow_moveing.Arrow_moveing_C" (`KismetMathLibrary.MakeTransform` (`SceneComponent.K2_GetComponentLocation` (`|GetArrayItem` (`|MakeArray` (`self.Up`) (`self.Right`) (`self.Left`) (`self.Down`)) (`self.RandomNum`))) (struct) (0.5 0.5 0.5)) "Undefined" "MultiplyWithRoot" null null))

(fn `UserConstructionScript`)