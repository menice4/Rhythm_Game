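; Player1Controls_BP handles input, pause and scoring for both players in an arrow-based game with timing ratings.
; BeginPlay shows the cursor and adds the Enhanced Input mapping, while the pause action toggles pause and calls the UI widget once the game starts.
; Rated-hit events add combo-multiplied points, raise the multiplier every ten hits and fire update calls; reset events clear combos.
; Directional inputs check game state and parent arrow type, but their branches are empty.
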(event `self.ReceiveBeginPlay`
  (bind _returnvalue (`GameplayStatics.GetPlayerController` 0))
  (bind _returnvalue_2 (pcsubsystem `EnhancedInputLocalPlayerSubsystem` _returnvalue))
  ;[1 1 1] Set Inputs
  (set `PlayerController.bShowMouseCursor` true _returnvalue)
  (cast `PlayerController` _returnvalue)
  (`/Engine/EditorBlueprintResources/StandardMacros.IsValid` _returnvalue_2
    (:`Is Valid`
      (`EnhancedInputSubsystemInterface.AddMappingContext` _returnvalue_2 "/Game/Inputs/ControlsInputMapping.ControlsInputMapping" 0 (struct)))))

(event `EnhancedInput|/Game/Inputs/IA_Pause`
  (params (ActionValue :type Boolean) (ElapsedSeconds :type "Float (double-precision)") (TriggeredSeconds :type "Float (double-precision)") (InputAction :type "InputAction Object Reference" :default "/Game/Inputs/IA_Pause.IA_Pause"))
  ;[1 1 1] Pause Input
  (:`Started`
    (bind _foundwidgets (`WidgetBlueprintLibrary.GetAllWidgetsOfClass` "/Game/Blueprints/UI.UI_C"))
    (if (`/Game/Blueprints/UI.GameStarted` (`|GetArrayItem` _foundwidgets))
      (if (`GameplayStatics.IsGamePaused`)
        (bind _foundwidgets_2 (`WidgetBlueprintLibrary.GetAllWidgetsOfClass` "/Game/Blueprints/UI.UI_C"))
        (`/Game/Blueprints/UI.ShowPause` (`|GetArrayItem` _foundwidgets_2))
        (`GameplayStatics.SetGamePaused` false)
        (else
          (bind _foundwidgets_3 (`WidgetBlueprintLibrary.GetAllWidgetsOfClass` "/Game/Blueprints/UI.UI_C"))
          (`/Game/Blueprints/UI.ShowPause` (`|GetArrayItem` _foundwidgets_3))
          (`GameplayStatics.SetGamePaused` true))))))

(event `EnhancedInput|/Game/Inputs/IA_Player1Down`
  (params (ActionValue :type Boolean) (ElapsedSeconds :type "Float (double-precision)") (TriggeredSeconds :type "Float (double-precision)") (InputAction :type "InputAction Object Reference" :default "/Game/Inputs/IA_Player1Down.IA_Player1Down"))
  (:`Started`
    (bind _foundwidgets (`WidgetBlueprintLibrary.GetAllWidgetsOfClass` "/Game/Blueprints/UI.UI_C"))
    (if (`/Game/Blueprints/UI.GameStarted` (`|GetArrayItem` _foundwidgets))
      (cast `/Game/Blueprints/Player1Arrow_BP` (`self.GetParentActor`))
      (if true
        _))))

(event `EnhancedInput|/Game/Inputs/IA_Player1Left`
  (params (ActionValue :type Boolean) (ElapsedSeconds :type "Float (double-precision)") (TriggeredSeconds :type "Float (double-precision)") (InputAction :type "InputAction Object Reference" :default "/Game/Inputs/IA_Player1Left.IA_Player1Left"))
  (:`Started`
    (bind _foundwidgets (`WidgetBlueprintLibrary.GetAllWidgetsOfClass` "/Game/Blueprints/UI.UI_C"))
    (if (`/Game/Blueprints/UI.GameStarted` (`|GetArrayItem` _foundwidgets))
      (cast `/Game/Blueprints/Player1Arrow_BP` (`self.GetParentActor`))
      (if true
        _))))

(event `EnhancedInput|/Game/Inputs/IA_Player1Right`
  (params (ActionValue :type Boolean) (ElapsedSeconds :type "Float (double-precision)") (TriggeredSeconds :type "Float (double-precision)") (InputAction :type "InputAction Object Reference" :default "/Game/Inputs/IA_Player1Right.IA_Player1Right"))
  (:`Started`
    (bind _foundwidgets (`WidgetBlueprintLibrary.GetAllWidgetsOfClass` "/Game/Blueprints/UI.UI_C"))
    (if (`/Game/Blueprints/UI.GameStarted` (`|GetArrayItem` _foundwidgets))
      (cast `/Game/Blueprints/Player1Arrow_BP` (`self.GetParentActor`))
      (if true
        _))))

(event `EnhancedInput|/Game/Inputs/IA_Player1Up`
  (params (ActionValue :type Boolean) (ElapsedSeconds :type "Float (double-precision)") (TriggeredSeconds :type "Float (double-precision)") (InputAction :type "InputAction Object Reference" :default "/Game/Inputs/IA_Player1Up.IA_Player1Up"))
  (:`Started`
    (bind _foundwidgets (`WidgetBlueprintLibrary.GetAllWidgetsOfClass` "/Game/Blueprints/UI.UI_C"))
    (if (`/Game/Blueprints/UI.GameStarted` (`|GetArrayItem` _foundwidgets))
      (cast `/Game/Blueprints/Player1Arrow_BP` (`self.GetParentActor`))
      (if true
        _))))

(event `IncreaseScoreGoodPlayer1`
  (bind _player1combo (`self.Player1Combo`))
  (bind _player1combocounter (`self.Player1ComboCounter`))
  ;[1 1 1] Score Mechanics Player 1
  (set `self.Player1Score` (+ (* 10 (`self.Player1Combo`)) (`self.Player1Score`)))
  (set `self.Player1ComboCounter` (+ 1 _player1combocounter) :!label _label)
  (`self.UpdatePlayer1Score` (`self.Player1Score`))
  (if (== _player1combocounter 10)
    (set `self.Player1Combo` (+ 1 _player1combo))
    (set `self.Player1ComboCounter` 0)
    (`self.UpdatePlayer1Combo` _player1combo)))

(event `IncreaseScoreExcellentPlayer1`
  ;[1 1 1] Score Mechanics Player 1
  (set `self.Player1Score` (+ (* 25 (`self.Player1Combo`)) (`self.Player1Score`)))
  (goto _label))

(event `IncreaseScorePerfectPlayer1`
  ;[1 1 1] Score Mechanics Player 1
  (set `self.Player1Score` (+ (* 50 (`self.Player1Combo`)) (`self.Player1Score`)))
  (goto _label))

(event `ResetComboPlayer1`
  ;[1 1 1] Score Mechanics Player 1
  (set `self.Player1Combo` 1)
  (set `self.Player1ComboCounter` 0)
  (`self.UpdatePlayer1Combo` (`self.Player1Combo`)))

(event `EnhancedInput|/Game/Inputs/IA_Player2Down`
  (params (ActionValue :type Boolean) (ElapsedSeconds :type "Float (double-precision)") (TriggeredSeconds :type "Float (double-precision)") (InputAction :type "InputAction Object Reference" :default "/Game/Inputs/IA_Player2Down.IA_Player2Down"))
  (:`Started`
    (bind _foundwidgets (`WidgetBlueprintLibrary.GetAllWidgetsOfClass` "/Game/Blueprints/UI.UI_C"))
    (bind _output (`|GetArrayItem` _foundwidgets))
    (if (and (`/Game/Blueprints/UI.GameStarted` _output) (`/Game/Blueprints/UI.2PlayerGame` _output))
      (cast `/Game/Blueprints/Player2Arrow_BP` (`self.GetParentActor`))
      (if true
        _))))

(event `EnhancedInput|/Game/Inputs/IA_Player2Left`
  (params (ActionValue :type Boolean) (ElapsedSeconds :type "Float (double-precision)") (TriggeredSeconds :type "Float (double-precision)") (InputAction :type "InputAction Object Reference" :default "/Game/Inputs/IA_Player2Left.IA_Player2Left"))
  (:`Started`
    (bind _foundwidgets (`WidgetBlueprintLibrary.GetAllWidgetsOfClass` "/Game/Blueprints/UI.UI_C"))
    (bind _output (`|GetArrayItem` _foundwidgets))
    (if (and (`/Game/Blueprints/UI.GameStarted` _output) (`/Game/Blueprints/UI.2PlayerGame` _output))
      (cast `/Game/Blueprints/Player2Arrow_BP` (`self.GetParentActor`))
      (if true
        _))))

(event `EnhancedInput|/Game/Inputs/IA_Player2Right`
  (params (ActionValue :type Boolean) (ElapsedSeconds :type "Float (double-precision)") (TriggeredSeconds :type "Float (double-precision)") (InputAction :type "InputAction Object Reference" :default "/Game/Inputs/IA_Player2Right.IA_Player2Right"))
  (:`Started`
    (bind _foundwidgets (`WidgetBlueprintLibrary.GetAllWidgetsOfClass` "/Game/Blueprints/UI.UI_C"))
    (bind _output (`|GetArrayItem` _foundwidgets))
    (if (and (`/Game/Blueprints/UI.GameStarted` _output) (`/Game/Blueprints/UI.2PlayerGame` _output))
      (cast `/Game/Blueprints/Player2Arrow_BP` (`self.GetParentActor`))
      (if true
        _))))

(event `EnhancedInput|/Game/Inputs/IA_Player2Up`
  (params (ActionValue :type Boolean) (ElapsedSeconds :type "Float (double-precision)") (TriggeredSeconds :type "Float (double-precision)") (InputAction :type "InputAction Object Reference" :default "/Game/Inputs/IA_Player2Up.IA_Player2Up"))
  (:`Started`
    (bind _foundwidgets (`WidgetBlueprintLibrary.GetAllWidgetsOfClass` "/Game/Blueprints/UI.UI_C"))
    (bind _output (`|GetArrayItem` _foundwidgets))
    (if (and (`/Game/Blueprints/UI.GameStarted` _output) (`/Game/Blueprints/UI.2PlayerGame` _output))
      (cast `/Game/Blueprints/Player2Arrow_BP` (`self.GetParentActor`))
      (if true
        _))))

(event `IncreaseScoreGoodPlayer2`
  (bind _player2combocounter (`self.Player2ComboCounter`))
  (bind _player2combo (`self.Player2Combo`))
  ;[1 1 1] Score Mechanics Player 2
  (set `self.Player2Score` (+ (* 10 (`self.Player2Combo`)) (`self.Player2Score`)))
  (set `self.Player2ComboCounter` (+ 1 _player2combocounter) :!label _label_2)
  (`self.UpdatePlayer2Score` (`self.Player2Score`))
  (if (== _player2combocounter 10)
    (set `self.Player2Combo` (+ 1 _player2combo))
    (set `self.Player2ComboCounter` 0)
    (`self.UpdatePlayer2Combo` _player2combo)))

(event `IncreaseScoreExcellentPlayer2`
  ;[1 1 1] Score Mechanics Player 2
  (set `self.Player2Score` (+ (* 25 (`self.Player2Combo`)) (`self.Player2Score`)))
  (goto _label_2))

(event `IncreaseScorePerfectPlayer2`
  ;[1 1 1] Score Mechanics Player 2
  (set `self.Player2Score` (+ (* 50 (`self.Player2Combo`)) (`self.Player2Score`)))
  (goto _label_2))

(event `ResetComboPlayer2`
  ;[1 1 1] Score Mechanics Player 2
  (set `self.Player2Combo` 1)
  (set `self.Player2ComboCounter` 0)
  (`self.UpdatePlayer2Combo` (`self.Player2Combo`)))

(fn `UserConstructionScript`)